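; BP_SceneController is the level's game-flow actor, running the HUD and win/lose screens.
; On BeginPlay it creates the gameplay HUD and a hidden endgame widget, passes the HUD the max time and interactable count, plays a sound and sets game-only input.
; CheckCounterStatus triggers GameWin once all interactions are collected.
; GameWin and GameLose show the endgame widget once, switch to UI input with cursor and hide the HUD.
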(event EventBeginPlay
  (CallFunction|SetWidgets)
  (CallFunction|InitializeWidgets)
  (Audio|PlaySound2D 0 1.0 1.0 0.0 0 0)
  (bind _returnvalue (Actor|GetActorOfClass "/Game/PrácticaGrupal/MainCharacter/BP_OwnCharacter.BP_OwnCharacter_C"))
  (Variables|Default|SetPlayer _returnvalue)
  (Input|SetInputModeGameOnly (Game|GetPlayerController 0) false))

(event Collision|EventActorBeginOverlap
  (params (OtherActor :type Actor%20Object%20Reference)))

(event EventTick
  (params (DeltaSeconds :type Float%20%28single-precision%29)))

(fn ConstructionScript)

(fn SetWidgets
  ;[1 1 1] Set Gameplay HUD
  (bind _returnvalue (UserInterface|CreateWidget "/Game/PrácticaGrupal/UI/Timer/WG_HUDGameplay.WG_HUDGameplay_C"))
  (bind _output_get (Variables|Default|SetHudGameplay _returnvalue))
  (UserInterface|Viewport|AddtoViewport _output_get 0)
  ;[1 1 1] Creating endgame widget but not showing yet
  (bind _returnvalue_2 (UserInterface|CreateWidget "/Game/PrácticaGrupal/UI/WG_endgame.WG_endgame_C"))
  (Variables|Default|SetEndgame _returnvalue_2))

(fn InitializeWidgets
  ;[1 1 1] Set max time of counter
  (Default|SetMaxTime (Variables|Default|GetHudGameplay) (Variables|Default|GetmaxTime))
  ;[1 1 1] Set Max Interactions item
  (bind _outactors (Actor|GetAllActorsOfClass "/Game/PrácticaGrupal/Interactions/Interactable/BP_Interactable_Base.BP_Interactable_Base_C"))
  (Default|SetMaxInteractions (Variables|Default|GetHudGameplay) (Utilities|Array|Length _outactors)))

(fn GameWin
  (bind _returnvalue (Game|GetPlayerController 0))
  (bind _endgame (Variables|Default|GetEndgame))
  ;[1 1 1] Avoid multiple widget screens & calls
  (if (not (Widget|IsVisible (Variables|Default|GetEndgame)))
    (Default|CallEndGame _endgame true) ; Set win status to widget
    (UserInterface|Viewport|AddtoViewport _endgame 0)
    (Variables|/Script/Engine.PlayerController|SetbShowMouseCursor _returnvalue true) ; Showing mouse in hud
    (Input|SetInputModeUIOnly _returnvalue _endgame "DoNotLock" true) ; setting UI only and restart value inputs
    (Widget|SetVisibility (Variables|Default|GetHudGameplay) "Hidden")))

(fn GameLose
  (bind _returnvalue (Game|GetPlayerController 0))
  (bind _endgame (Variables|Default|GetEndgame))
  ;[1 1 1] Avoid multiple widget screens & calls
  (if (not (Widget|IsVisible (Variables|Default|GetEndgame)))
    (Default|CallEndGame _endgame false) ; Setting lose status to widget
    (UserInterface|Viewport|AddtoViewport _endgame 0)
    (Variables|/Script/Engine.PlayerController|SetbShowMouseCursor _returnvalue true)
    (Input|SetInputModeUIOnly _returnvalue _endgame "DoNotLock" true)
    (Widget|SetVisibility (Variables|Default|GetHudGameplay) "Hidden")))

(fn CheckCounterStatus
  (bind _hudgameplay (Variables|Default|GetHudGameplay))
  ;[1 1 1] Check if player has all items, and if its true, player wins
  (if (>= (Variables|/Game/PrácticaGrupal/UI/Timer/WG_HUDGameplay.WG_HUDGameplay_C|GetCurrent%20Interactions _hudgameplay) (Variables|/Game/PrácticaGrupal/UI/Timer/WG_HUDGameplay.WG_HUDGameplay_C|GetMax%20Interaction _hudgameplay))
    (CallFunction|GameWin)))