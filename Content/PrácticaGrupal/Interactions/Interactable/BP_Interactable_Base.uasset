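; Base Blueprint for pickable interactables that show a prompt widget while the player pawn overlaps them.
; The Pick event acts only while the widget is visible, adding to the scene controller's interaction counter, triggering its status check, then destroying the actor.
; It finds the BP_SceneController at BeginPlay.
; A ShowLight helper toggles a point light, but its calls in the event graph are unconnected.
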(event EventBeginPlay
  (bind _outactors (Actor|GetAllActorsOfClass "/Game/BluePrints/BP_SceneController.BP_SceneController_C"))
  (Variables|Default|SetSceneController (Utilities|Array|Get(acopy) _outactors))
  (Rendering|SetVisibility (Variables|Default|GetWidget) false false))

(event EventPick
  (CallFunction|DoPick))

(event Collision|EventActorEndOverlap
  (params (OtherActor :type Actor%20Object%20Reference))
  (bind _isplayer (CallFunction|IsPlayer OtherActor))
  (if _isplayer
    (CallFunction|SetVisual false)))

(event Collision|EventActorBeginOverlap
  (params (OtherActor :type Actor%20Object%20Reference))
  (bind _isplayer (CallFunction|IsPlayer OtherActor))
  (if _isplayer
    (CallFunction|SetVisual true)))

(fn ConstructionScript)

(fn SetVisual
  (params (IsVisible :type Boolean))
  (Rendering|SetVisibility (Variables|Default|GetWidget) IsVisible false))

(fn IsPlayer
  (params (OtherActor :type Actor%20Object%20Reference))
  (return (== OtherActor (Game|Player|GetPlayerPawn 0))))

(fn DoPick
  (bind _scenecontroller (Variables|Default|GetSceneController))
  (if (Rendering|IsVisible (Variables|Default|GetWidget))
    (Default|AddInteraction (Variables|/Game/BluePrints/BP_SceneController.BP_SceneController_C|GetInteractableCounter _scenecontroller))
    (Default|CheckCounterStatus _scenecontroller)
    (Actor|DestroyActor)))

(fn ShowLight
  (params (Show :type Boolean))
  (Rendering|SetVisibility (Variables|Default|GetPointLight) Show false))