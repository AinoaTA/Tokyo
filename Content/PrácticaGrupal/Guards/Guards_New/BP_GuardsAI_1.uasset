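; Guard AI that chases the player once PawnSensing spots a pawn, issuing an arrest warning by text and sound as pursuit starts.
; After reaching the player, it waits, moves to a random reachable navmesh point, then sets its rotation from the player's transform.
; OnUnseePawn clears the sighting flag and recalls it to BP_GuardZone_1, though nothing here calls that event.
; The overlap handlers are empty, and several older branches, including GameLose, are disconnected.
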(event OnSeePawn(PawnSensing)
  (params (Pawn :type Pawn%20Object%20Reference))
  ;[1 1 1] Event Start Look for the Player
  (Variables|Default|SetisSeeingPlayer true)
  (Utilities|FlowControl|Delay 1.5)
  (CallFunction|FollowPlayer))

(event Custom|CustomEvent_1
  (params (OverlappedActor :type Actor%20Object%20Reference) (OtherActor :type Actor%20Object%20Reference))
  ;[0 0.8887 1] Guard Pursuit and get back to random zone in the navmesh
)

(event Custom|FollowPlayer
  ;[0 0.8887 1] Guard Pursuit and get back to random zone in the navmesh
  (if (Variables|Default|GetisSeeingPlayer)
    (AI|AIMoveTo self "0, 0, 0" (Game|GetPlayerCharacter 0) 5.0 true
      (:then
        (EventDispatchers|AssignOnActorBeginOverlap (delegate Custom|CustomEvent_1))
        (Development|PrintText "Get On the Floor. You are under arrest!")
        (Utilities|FlowControl|Delay 1.0)
        (Audio|PlaySound2D "/Game/TokyoStylizedEnvironment/Audio/Ambient/human_male_uk_police_officer_says_get_on_the_floor_your_under_arrest_001_44265.human_male_uk_police_officer_says_get_on_the_floor_your_under_arrest_001_44265" 1.0 1.0 0.0 0 0))
      (:OnSuccess
        (Utilities|FlowControl|Delay 5.0)
        (AI|AIMoveTo self (.RandomLocation (AI|Navigation|GetRandomReachablePointinRadius (Transformation|GetActorLocation) (Variables|Default|GetRadius) 0 0)) 0 (Variables|Default|GetAcceptance%20Radius) true
          (:OnSuccess
            (Utilities|FlowControl|Delay 8.0)
            (CallFunction|RotateGuard)))))))

(event Custom|OnUnseePawn
  ;[1 1 1] Sandbox
  (Variables|Default|SetisSeeingPlayer false)
  (Utilities|FlowControl|Delay 0.2)
  (CallFunction|RecalltoBase))

(event Custom|RecallToBase
  ;[1 1 1] Sandbox
  (if (not (Variables|Default|GetisSeeingPlayer))
    (Utilities|FlowControl|Delay 5.0)
    (bind _returnvalue (Actor|GetActorOfClass "/Game/PrácticaGrupal/Guards/Guards_New/BP_GuardZone_1.BP_GuardZone_1_C"))
    (AI|AIMoveTo self "0, 0, 0" _returnvalue 5.0 false)))

(event Custom|OnActorBeginOverlap_Event
  (params (OverlappedActor :type Actor%20Object%20Reference) (OtherActor :type Actor%20Object%20Reference))
  ;[1 1 1] Guard Pursuit and get back to the exact zone
)

(event EventBeginPlay)

(event Collision|EventActorBeginOverlap
  (params (OtherActor :type Actor%20Object%20Reference)))

(event EventTick
  (params (DeltaSeconds :type Float%20%28single-precision%29)))

(fn ConstructionScript)

(fn RotateGuard
  (bind _returnvalue (Game|GetPlayerCharacter 0))
  (bind _returnvalue_2 (Transformation|GetActorTransform _returnvalue))
  (bind _returnvalue_3 (Math|Transform|TransformRotation _returnvalue_2 "-180.000000,-180.000000,180.000000"))
  ;[1 1 1] Rotate the Guard to look forward
  (Development|PrintText (Utilities|Text|ToText(String) _returnvalue_3) true true "(R=0.000000,G=0.660000,B=1.000000,A=1.000000)" 3e+01)
  (Transformation|SetActorRotation self _returnvalue_3))