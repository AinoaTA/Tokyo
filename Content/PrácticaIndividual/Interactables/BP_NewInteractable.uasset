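; BP_NewInteractable is a pickup item that shows a prompt widget while the player overlaps it.
; Each tick, the visible widget turns toward the player, keeping its pitch.
; Interact works only while the widget shows: it deregisters the item, updates the HUD, has BP_SceneController check collection progress, plays a sound and destroys itself.
; Init caches the scene controller and hides the widget; ShowLight toggles a point light.
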(event EventInteract
  (CallFunction|DoPick))

(event EventTick
  (params (DeltaSeconds :type Float%20%28single-precision%29))
  (CallFunction|Lookat))

(event EventNextBeginPlay
  (CallFunction|Init))

(event Collision|EventActorEndOverlap
  (params (OtherActor :type Actor%20Object%20Reference))
  (bind _isplayer (CallFunction|IsPlayer OtherActor))
  (if _isplayer
    (CallFunction|SetVisual false)))

(event Collision|EventActorBeginOverlap
  (params (OtherActor :type Actor%20Object%20Reference))
  (bind _isplayer (CallFunction|IsPlayer OtherActor))
  (if _isplayer
    (CallFunction|SetVisual true)))

(fn ConstructionScript)

(fn Lookat
  (bind _returnvalue (Game|Player|GetPlayerPawn 0))
  (bind _widget (Variables|Default|GetWidget))
  (bind _returnvalue_2 (Transformation|GetWorldLocation _widget))
  (bind _returnvalue_3 (Transformation|GetActorLocation _returnvalue))
  (bind _returnvalue_4 (Math|Rotator|FindLookatRotation _returnvalue_2 _returnvalue_3))
  (if (Rendering|IsVisible (Variables|Default|GetWidget))
    (Transformation|SetWorldRotation (Variables|Default|GetWidget) (Math|Rotator|MakeRotator (.roll _returnvalue_4) (.pitch (Transformation|GetWorldRotation (Variables|Default|GetWidget))) (.yaw _returnvalue_4)) false false)))

(fn SetVisual
  (params (Is%20Visible :type Boolean))
  ;[1 1 1] Show user widget
  (Rendering|SetVisibility (Variables|Default|GetWidget) Is%20Visible false))

(fn IsPlayer
  (params (Other%20Actor :type Actor%20Object%20Reference))
  (return (== Other%20Actor (Game|Player|GetPlayerPawn 0))))

(fn DoPick
  (bind _self self)
  (bind _scene_controller (Variables|Default|GetScene%20Controller))
  (if (Rendering|IsVisible (Variables|Default|GetWidget))
    (Class|InteractableInput|RemoveInteractablefromManager _self _self)
    (Default|AddInteraction (Variables|/Game/PrácticaGrupal/Settings/BP_SceneController.BP_SceneController_C|GetHudGameplay _scene_controller))
    (Default|CheckCounterStatus _scene_controller) ; Check if player has all items
    (Audio|PlaySound2D "/Game/PrácticaIndividual/SFX/sfx_pickupitem.sfx_pickupitem" 1.0 1.0 0.0 0 0)
    (Actor|DestroyActor)))

(fn ShowLight
  (params (Show :type Boolean))
  (Rendering|SetVisibility (Variables|Default|GetPointLight) Show false))

(fn Init
  (bind _outactors (Actor|GetAllActorsOfClass "/Game/PrácticaGrupal/Settings/BP_SceneController.BP_SceneController_C"))
  (Variables|Default|SetScene%20Controller (Utilities|Array|Get(acopy) _outactors))
  (Rendering|SetVisibility (Variables|Default|GetWidget) false false)
  (Actor|GetActorOfClass 0))