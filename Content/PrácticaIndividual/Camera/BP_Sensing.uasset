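; BP_Sensing is the detection part of a security camera, spotting the player character and switching the camera between follow and patrol colors.
; It receives its camera reference through Initialize, and PawnSensing's OnSeePawn sets the seeing flag, triggers the follow color and prints debug text.
; While the flag is set, Tick restores the patrol color once the camera-to-player distance reaches the sight radius, so losing sight depends only on distance.
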(event OnSeePawn(PawnSensing)
  (params (Pawn :type Pawn%20Object%20Reference))
  (bind _camera (Variables|Default|GetCamera))
  (bind _asbp_own_character (Utilities|Casting|CastToBP_OwnCharacter Pawn))
  (Development|PrintString "Hello")
  (bind _output_get (Variables|Default|SetIsSeeingPlayer true))
  (Development|PrintString (Utilities|String|ToString(Boolean) _output_get))
  (Default|FollowSetColor _camera)
  (Development|PrintString (Utilities|String|ToString(Float) (Transformation|GetDistanceTo _camera 0))))

(event EventBeginPlay)

(event Collision|EventActorBeginOverlap
  (params (OtherActor :type Actor%20Object%20Reference)))

(event EventTick
  (params (DeltaSeconds :type Float%20%28single-precision%29))
  (if (Variables|Default|GetIsSeeingPlayer)
    (if (>= (Transformation|GetDistanceTo (Variables|Default|GetCamera) (stale OnSeePawn(PawnSensing) _asbp_own_character)) (Variables|/Script/AIModule.PawnSensingComponent|GetSightRadius (Variables|Default|GetPawnSensing)))
      (Variables|Default|SetIsSeeingPlayer false)
      (Default|PatrolSetColor (Variables|Default|GetCamera)))))

(fn ConstructionScript)

(fn Initialize
  (params (bp_cam :type BP%20Camera%20Object%20Reference))
  (Variables|Default|SetCamera bp_cam))