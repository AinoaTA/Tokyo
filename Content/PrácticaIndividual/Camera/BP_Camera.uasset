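; BP_Camera is a security camera that sweeps an area and turns to track the player when its sensor sees them.
; It initializes a BP_Sensing child actor with itself and reads that actor's IsSeeingPlayer flag every Tick.
; While seen, the mesh yaws toward the player; otherwise a Timeline drives the patrol sweep.
; FollowSetColor and PatrolSetColor switch the spotlight color but are not called within this Blueprint.
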(event EventBeginPlay
  (Variables|Default|SetPlayer (Game|GetPlayerCharacter 0))
  (bind _asbp_sensing (Utilities|Casting|CastToBP_Sensing (Variables|/Script/Engine.ChildActorComponent|GetChildActor (Variables|Default|GetBP_sensing))))
  (bind _output_get (Variables|Default|SetSensing _asbp_sensing))
  (Default|Initialize _output_get self))

(event Collision|EventActorBeginOverlap
  (params (OtherActor :type Actor%20Object%20Reference)))

(event EventTick
  (params (DeltaSeconds :type Float%20%28single-precision%29))
  (bind _staticmesh (Variables|Default|GetStaticMesh))
  (bind _staticmesh_2 (Variables|Default|GetStaticMesh))
  (bind _returnvalue (Transformation|GetWorldRotation _staticmesh))
  (bind _returnvalue_2 (Transformation|GetWorldRotation _staticmesh_2))
  (if (Variables|/Game/PrácticaIndividual/Camera/BP_Sensing.BP_Sensing_C|GetIsSeeingPlayer (Variables|Default|GetSensing))
    (Transformation|SetWorldRotation (Variables|Default|GetStaticMesh) (Math|Rotator|MakeRotator (.roll _returnvalue_2) (.pitch _returnvalue_2) (+ (.yaw (Math|Rotator|FindLookatRotation (Transformation|GetWorldLocation (Variables|Default|GetStaticMesh)) (Transformation|GetActorLocation (Game|Player|GetPlayerPawn 0)))) -9e+01)) false false)
    (Development|PrintString "roting")
    (bind _rotation (Timeline|Timeline Stop)
      (:Update
        (Transformation|SetRelativeRotation _staticmesh (Math|Rotator|MakeRotator (.roll _returnvalue) (.pitch _returnvalue) (* _rotation 75.0)) false false)))
    (else
      (Timeline|Timeline Play))))

(fn ConstructionScript)

(fn FollowSetColor
  (Rendering|Components|Light|SetLightColor (Variables|Default|GetSpotLight) (Math|Conversions|ToLinearColor(Color) (Variables|Default|GetFollowColor)) false))

(fn PatrolSetColor
  (Rendering|Components|Light|SetLightColor (Variables|Default|GetSpotLight) (Math|Conversions|ToLinearColor(Color) (Variables|Default|GetPatrolColor)) false))