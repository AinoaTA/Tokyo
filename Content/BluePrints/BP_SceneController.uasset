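; BP_SceneController sets up the level's HUD and holds stub win and lose handlers for the game.
; On BeginPlay it creates the interactable counter and timer widgets, adds them to the viewport, then passes MaxInteractions and MaxTime into them.
; GameWin is empty and GameLose only prints a debug string; nothing in this Blueprint calls either function.
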(event EventBeginPlay
  (CallFunction|SetWidgets)
  (CallFunction|InitializeWidgets))

(event Collision|EventActorBeginOverlap
  (params (OtherActor :type Actor%20Object%20Reference)))

(event EventTick
  (params (DeltaSeconds :type Float%20%28single-precision%29)))

(fn ConstructionScript)

(fn SetWidgets
  (bind _returnvalue (UserInterface|CreateWidget "/Game/BluePrints/Interactable/WG_Interctables.WG_Interctables_C"))
  (bind _output_get (Variables|Default|SetInteractableCounter _returnvalue))
  (UserInterface|Viewport|AddtoViewport _output_get 0)
  (bind _returnvalue_2 (UserInterface|CreateWidget "/Game/BluePrints/Interactable/Timer/WG_Timer.WG_Timer_C"))
  (bind _output_get_2 (Variables|Default|SetTimer _returnvalue_2))
  (UserInterface|Viewport|AddtoViewport _output_get_2 0))

(fn InitializeWidgets
  (Default|SetMaxInteractions (Variables|Default|GetInteractableCounter) (Variables|Default|GetmaxInteractions))
  (Default|SetMaxTime (Variables|Default|GetTimer) (Variables|Default|GetmaxTime)))

(fn GameWin)

(fn GameLose
  (Development|PrintString "Game lost"))