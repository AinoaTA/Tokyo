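; BP_Interactable_Weapon is an interactable weapon pickup that the player can collect when nearby.
; Player pawn overlap toggles a prompt widget and a point light, with the widget hidden on BeginPlay.
; The Pick event only succeeds while the widget is visible, using that visibility as a proximity check.
; A successful pick adds an interaction to the InteractableCounter of the BP_SceneController found at BeginPlay, then destroys the actor.
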(event EventBeginPlay
  (bind _outactors (Actor|GetAllActorsOfClass "/Game/BluePrints/BP_SceneController.BP_SceneController_C"))
  (Variables|Default|SetSceneController (Utilities|Array|Get(acopy) _outactors))
  (Rendering|SetVisibility (Variables|Default|GetWidget) false false))

(event EventPick
  (CallFunction|DoPick))

(event Collision|EventActorEndOverlap
  (params (OtherActor :type Actor%20Object%20Reference))
  (bind _isplayer (CallFunction|IsPlayer OtherActor))
  (if _isplayer
    (CallFunction|SetVisual false)
    (CallFunction|ShowLight false)))

(event Collision|EventActorBeginOverlap
  (params (OtherActor :type Actor%20Object%20Reference))
  (bind _isplayer (CallFunction|IsPlayer OtherActor))
  (if _isplayer
    (CallFunction|SetVisual true)
    (CallFunction|ShowLight true)))

(fn ConstructionScript)

(fn SetVisual
  (params (IsVisible :type Boolean))
  (Rendering|SetVisibility (Variables|Default|GetWidget) IsVisible false))

(fn IsPlayer
  (params (OtherActor :type Actor%20Object%20Reference))
  (return (== OtherActor (Game|Player|GetPlayerPawn 0))))

(fn DoPick
  (if (Rendering|IsVisible (Variables|Default|GetWidget))
    (Default|AddInteraction (Variables|/Game/BluePrints/BP_SceneController.BP_SceneController_C|GetInteractableCounter (Variables|Default|GetSceneController)))
    (Actor|DestroyActor)))

(fn ShowLight
  (params (Show :type Boolean))
  (Rendering|SetVisibility (Variables|Default|GetPointLight) Show false))