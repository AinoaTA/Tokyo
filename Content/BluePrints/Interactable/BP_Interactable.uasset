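; BP_Interactable is a pickup actor that counts as an interaction when the player collects it.
; On BeginPlay it caches the first BP_SceneController found in the level.
; When the player pawn overlaps it, the Pick event adds an interaction to that controller's Counter and destroys the actor.
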(event EventBeginPlay
  (bind _outactors (Actor|GetAllActorsOfClass "/Game/BluePrints/BP_SceneController.BP_SceneController_C"))
  (Variables|Default|SetSceneController (Utilities|Array|Get(acopy) _outactors)))

(event Collision|EventActorBeginOverlap
  (params (OtherActor :type Actor%20Object%20Reference))
  (if (== OtherActor (Game|Player|GetPlayerPawn 0))
    (CallFunction|Pick)))

(event EventTick
  (params (DeltaSeconds :type Float%20%28single-precision%29)))

(event EventPick
  (Default|AddInteraction (Variables|/Game/BluePrints/BP_SceneController.BP_SceneController_C|GetCounter (Variables|Default|GetSceneController)))
  (Actor|DestroyActor))

(fn ConstructionScript)