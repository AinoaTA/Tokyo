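; BP_GuardsAI is a guard AI that chases the player once it spots them.
; PawnSensing sets a seen flag and, after a short delay, calls FollowPlayer, which issues AI MoveTo toward the player character.
; The MoveTo's immediate output, not its success, binds an empty overlap handler, prints a caught message and plays a delayed police arrest voice line.
; The seen flag is never cleared here.
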(event OnSeePawn(PawnSensing)
  (params (Pawn :type Pawn%20Object%20Reference))
  (Variables|Default|SetisSeeingPlayer true)
  (Utilities|FlowControl|Delay 1.5)
  (CallFunction|FollowPlayer))

(event Custom|FollowPlayer
  (if (Variables|Default|GetisSeeingPlayer)
    (AI|AIMoveTo self "0, 0, 0" (Game|GetPlayerCharacter 0) 5.0 true
      (:then
        (EventDispatchers|AssignOnActorBeginOverlap (delegate Custom|OnActorBeginOverlap_Event))
        (Development|PrintText "I've got you!!!!")
        (Utilities|FlowControl|Delay 1.0)
        (Audio|PlaySound2D "/Game/TokyoStylizedEnvironment/Audio/Ambient/human_male_uk_police_officer_says_get_on_the_floor_your_under_arrest_001_44265.human_male_uk_police_officer_says_get_on_the_floor_your_under_arrest_001_44265" 1.0 1.0 0.0 0 0)))))

(event Custom|OnActorBeginOverlap_Event
  (params (OverlappedActor :type Actor%20Object%20Reference) (OtherActor :type Actor%20Object%20Reference)))

(event EventBeginPlay)

(event Collision|EventActorBeginOverlap
  (params (OtherActor :type Actor%20Object%20Reference)))

(event EventTick
  (params (DeltaSeconds :type Float%20%28single-precision%29)))

(fn ConstructionScript)